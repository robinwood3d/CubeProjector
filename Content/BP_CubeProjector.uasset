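; Cube projector actor that projects an image or runtime-supplied texture onto the surrounding scene through a decal, with an optional background sphere.
; Construction builds dynamic materials for decal and sphere from ProjectionSettings and scales the decal to projection distance.
; Optional depth comes from a SceneCaptureCube rendering into a created cube render target.
; Tick feeds actor axes to both materials; SetProjectionTexture recaptures and swaps only the decal's image.
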(event `self.ReceiveTick`
  (params (DeltaSeconds :type "Float (single-precision)"))
  (`self.UpdateCubeAxis`))

(event `self.SceneCaptureComponentCube.OnComponentActivated`
  (params (Component :type "ActorComponent Object Reference") (bReset :type Boolean))
  (`KismetSystemLibrary.Delay` 0.2)
  (`SceneCaptureComponentCube.CaptureScene` (`self.SceneCaptureComponentCube`)))

(fn `SetProjectionTexture`
  (params (Texture :type "Texture Object Reference"))
  (`SceneCaptureComponentCube.CaptureScene` (`self.SceneCaptureComponentCube`))
  (`MaterialInstanceDynamic.SetTextureParameterValue` (`self.ProjectionMID`) "Image" Texture))

(fn `UpdateCubeAxis`
  (bind _projectionmid (`self.ProjectionMID`)
    (:`then`
      (`MaterialInstanceDynamic.SetVectorParameterValue` _projectionmid "X" (`KismetMathLibrary.Conv_VectorToLinearColor` (`self.GetActorForwardVector`)))
      (`MaterialInstanceDynamic.SetVectorParameterValue` (`self.BackgroundMID`) "X" (`KismetMathLibrary.Conv_VectorToLinearColor` (`self.GetActorForwardVector`)))
      (`MaterialInstanceDynamic.SetVectorParameterValue` (`self.ProjectionMID`) "Y" (`KismetMathLibrary.Conv_VectorToLinearColor` (`self.GetActorRightVector`)))
      (`MaterialInstanceDynamic.SetVectorParameterValue` (`self.BackgroundMID`) "Y" (`KismetMathLibrary.Conv_VectorToLinearColor` (`self.GetActorRightVector`)))
      (`MaterialInstanceDynamic.SetVectorParameterValue` (`self.ProjectionMID`) "Z" (`KismetMathLibrary.Conv_VectorToLinearColor` (`self.GetActorUpVector`)))
      (`MaterialInstanceDynamic.SetVectorParameterValue` (`self.BackgroundMID`) "Z" (`KismetMathLibrary.Conv_VectorToLinearColor` (`self.GetActorUpVector`))))
    (:`else`)))

(fn `UpdateProjection`
  (bind _scenecapturecomponentcube (`self.SceneCaptureComponentCube`))
  (bind _scenecapturecomponentcube_2 (`self.SceneCaptureComponentCube`))
  (bind ((`DepthBias_51_0526F894424F344CF062DEAA0CFDC0EF` _depthbias) (`Gamma_52_44EFAA594F569E5DF355BA8602178DD0` _gamma) (`Brightness_53_C7615E844AA35FF983EE9B8586AD00A4` _brightness)) (break `/CubeProjector/CubeProjectionSettings` (`self.ProjectionSettings`)))
  (setmembers `/CubeProjector/CubeProjectionSettings` :`StructRef` (`self.ProjectionSettings`) :`ProjectOrigin` (`self.K2_GetActorLocation`) :`ProjectRotator` (`self.K2_GetActorRotation`))
  (`|ExecutionSequence`
    (:`then_0`
      (`SceneComponent.SetWorldScale3D` (`self.Decal`) (`KismetMathLibrary.Conv_DoubleToVector` (`.ProjectDistance_50_A6317325454A3E7AA248029F29849DF9` (break `/CubeProjector/CubeProjectionSettings` (`self.ProjectionSettings`))))))
    (:`then_1`
      (bind _returnvalue (`KismetMaterialLibrary.CreateDynamicMaterialInstance` "/CubeProjector/Materials/M_CubeProjection.M_CubeProjection"))
      (set `self.ProjectionMID` _returnvalue)
      (bind _returnvalue_2 (`KismetMaterialLibrary.CreateDynamicMaterialInstance` "/CubeProjector/Materials/M_BackgrounSphere.M_BackgrounSphere"))
      (set `self.BackgroundMID` _returnvalue_2)
      (`MaterialInstanceDynamic.SetTextureParameterValue` (`self.ProjectionMID`) "Image" (`self.PreviewImage`))
      (`MaterialInstanceDynamic.SetTextureParameterValue` (`self.BackgroundMID`) "Image" (`self.PreviewImage`))
      (`MaterialInstanceDynamic.SetScalarParameterValue` (`self.ProjectionMID`) "DepthBias" _depthbias)
      (`MaterialInstanceDynamic.SetScalarParameterValue` (`self.BackgroundMID`) "DepthBias" _depthbias)
      (`MaterialInstanceDynamic.SetScalarParameterValue` (`self.ProjectionMID`) "Gamma" _gamma)
      (`MaterialInstanceDynamic.SetScalarParameterValue` (`self.BackgroundMID`) "Gamma" _gamma)
      (`MaterialInstanceDynamic.SetScalarParameterValue` (`self.ProjectionMID`) "Brightness" _brightness)
      (`MaterialInstanceDynamic.SetScalarParameterValue` (`self.BackgroundMID`) "Brightness" _brightness)
      (`MaterialInstanceDynamic.SetScalarParameterValue` (`self.ProjectionMID`) "EnableDepth" 1.0)
      (`MaterialInstanceDynamic.SetScalarParameterValue` (`self.BackgroundMID`) "EnableDepth" 1.0)
      (`MaterialInstanceDynamic.SetScalarParameterValue` (`self.ProjectionMID`) "ProjectDistance" (`.ProjectDistance_50_A6317325454A3E7AA248029F29849DF9` (break `/CubeProjector/CubeProjectionSettings` (`self.ProjectionSettings`))))
      (`self.UpdateCubeAxis`)
      (`DecalComponent.SetDecalMaterial` (`self.Decal`) (`self.ProjectionMID`))
      (`PrimitiveComponent.SetMaterial` (`self.Background`) 0 (`self.BackgroundMID`)))
    (:`then_2`
      (if (`.bEnableDepth_49_77AA248E4A1FAB3AD9AF8AB22DA97EBD` (break `/CubeProjector/CubeProjectionSettings` (`self.ProjectionSettings`)))
        (bind _returnvalue_3 (`CubeProjectorBPLibrary.CreateRenderTargetCube` (`.DepthSize_41_4D03C3BD4162D09E379354A9AF54FD6A` (break `/CubeProjector/CubeProjectionSettings` (`self.ProjectionSettings`)))))
        (bind _output_get (set `SceneCaptureComponentCube.TextureTarget` _returnvalue_3 (`self.SceneCaptureComponentCube`)))
        (`MaterialInstanceDynamic.SetTextureParameterValue` (`self.ProjectionMID`) "Depth" _output_get)
        (`MaterialInstanceDynamic.SetTextureParameterValue` (`self.BackgroundMID`) "Depth" _output_get)
        (set `SceneCaptureComponent.bCaptureOnMovement` true _scenecapturecomponentcube)
        (set `SceneCaptureComponent.bCaptureEveryFrame` (`.bUpdateDepthEveryFrame_47_8623FFF540F41B1C98BFD4AE861B2C04` (break `/CubeProjector/CubeProjectionSettings` (`self.ProjectionSettings`))) _scenecapturecomponentcube)
        (else
          (set `SceneCaptureComponent.bCaptureOnMovement` false _scenecapturecomponentcube_2)
          (set `SceneCaptureComponent.bCaptureEveryFrame` false _scenecapturecomponentcube_2)
          (`MaterialInstanceDynamic.SetScalarParameterValue` (`self.ProjectionMID`) "EnableDepth" 0.0)
          (`MaterialInstanceDynamic.SetScalarParameterValue` (`self.BackgroundMID`) "EnableDepth" 0.0))))
    (:`then_3`
      (`SceneComponent.SetVisibility` (`self.Background`) (`.bUseBackgroundSphere_56_FF1BC9D64F2A57FB5DEE3CA4AD6BDEC1` (break `/CubeProjector/CubeProjectionSettings` (`self.ProjectionSettings`))) false))))

(fn `UserConstructionScript`
  (`self.UpdateProjection`))